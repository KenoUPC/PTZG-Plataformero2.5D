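; Base moving platform that slides its Cube between the actor's location and that location offset by FinalPoint.
; A Timeline track supplies the alpha to InterpPlatformLocation, which lerps the Cube's world position without sweeping while the actor stays put as the anchor.
; When PingPong is set, movement starts on BeginPlay.
; Once started, the Timeline's Finished output alternates between ReverseMovement and StartMovement, looping the motion indefinitely.
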(event Custom|Start%20Movement
  (bind (_direction _pinpong) (Timeline|Timeline PlayFromStart)
    (:Update
      (CallFunction|InterpPlatformLocation _pinpong))
    (:Finished
      (switch Utilities|FlowControl|Switch|SwitchonETimelineDirection _direction
        (:Forward
          (CallFunction|ReverseMovement))
        (:Backward
          (CallFunction|StartMovement))))))

(event Custom|Reverse%20Movement
  (bind (_direction _pinpong) (Timeline|Timeline ReverseFromEnd)
    (:Update
      (CallFunction|InterpPlatformLocation _pinpong))
    (:Finished
      (switch Utilities|FlowControl|Switch|SwitchonETimelineDirection _direction
        (:Forward
          (CallFunction|ReverseMovement))
        (:Backward
          (CallFunction|StartMovement))))))

(event EventBeginPlay
  (if (Variables|Default|GetbPingPong?)
    (CallFunction|StartMovement)))

(event Collision|EventActorBeginOverlap
  (params (OtherActor :type Actor%20Object%20Reference)))

(event EventTick
  (params (DeltaSeconds :type Float%20%28single-precision%29)))

(fn ConstructionScript)

(fn InterpPlatformLocation
  (params (Alpha :type Float%20%28double-precision%29))
  (Transformation|SetWorldLocation (Variables|Default|GetCube) (Math|Vector|Lerp(Vector) (Transformation|GetActorLocation) (+ (Transformation|GetActorLocation) (Variables|Default|GetFinalPoint)) Alpha) false false))