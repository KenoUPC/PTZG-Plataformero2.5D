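; Spike trap actor (pinches) that periodically thrusts out and retracts, damaging and launching players it touches.
; A looping timer plays a timeline that sweeps the Box from the actor's starting location by the Posicion world-space offset, then reverses it after a short pause.
; On overlap, the Box damages actors implementing the BP_Player interface and sends them ForceImpulse through an interface launch message.
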(event OnComponentBeginOverlap(Box)
  (params (OverlappedComponent :type Primitive%20Component%20Object%20Reference) (OtherActor :type Actor%20Object%20Reference) (OtherComp :type Primitive%20Component%20Object%20Reference) (OtherBodyIndex :type Integer) (bFromSweep :type Boolean) (SweepResult :type Hit%20Result%20Structure%20%28by%20ref%29))
  (if (Utilities|DoesObjectImplementInterface OtherActor "/Game/Interfaces/BP_Player.BP_Player_C")
    (Game|Damage|ApplyDamage OtherActor 1.0 0 0)
    (Class|BPPlayer|ForceLauncher(Message) OtherActor (Variables|Default|GetForceImpulse))))

(event Custom|Reverse
  (bind (_direction _newtrack_0) (Timeline|Picnhes ReverseFromEnd)
    (:Update
      (CallFunction|MovePinches _newtrack_0))
    (:Finished
      (switch Utilities|FlowControl|Switch|SwitchonETimelineDirection _direction
        (:Forward
          (Utilities|FlowControl|Delay 0.1)
          (CallFunction|Reverse))))))

(event Custom|Start
  (bind (_direction _newtrack_0) (Timeline|Picnhes Play)
    (:Update
      (CallFunction|MovePinches _newtrack_0))
    (:Finished
      (switch Utilities|FlowControl|Switch|SwitchonETimelineDirection _direction
        (:Forward
          (Utilities|FlowControl|Delay 0.1)
          (CallFunction|Reverse))))))

(event EventBeginPlay
  (Variables|Default|SetInitPos (Transformation|GetActorLocation))
  (Utilities|Time|SetTimerbyEvent (delegate Custom|Start) 3.0 true))

(event EventTick
  (params (DeltaSeconds :type Float%20%28single-precision%29)))

(fn ConstructionScript)

(fn MovePinches
  (params (Alpha :type Float%20%28double-precision%29))
  (bind _initpos (Variables|Default|GetInitPos))
  (Transformation|SetWorldLocation (Variables|Default|GetBox) (Math|Vector|Lerp(Vector) _initpos (+ _initpos (Variables|Default|GetPosicion)) Alpha) true false))