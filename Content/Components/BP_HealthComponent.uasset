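; BP_HealthComponent is a health component that tracks current and maximum health for its owner.
; DecressHealth prints a debug string, lowers CurrentHealth by one, and broadcasts the new value through UpdateDamgeRecive.
; When health equals exactly zero it also calls Dead after that update.
; GetInitHealthData returns the max and current values.
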(fn DecressHealth
  (bind _currenthealth (Variables|Default|GetCurrentHealth))
  (Development|PrintString "Hello")
  (Math|Integer|DecrementInt (Variables|Default|GetCurrentHealth)
    (:%20%20
      (if (== (Variables|Default|GetCurrentHealth) 0)
        (Default|CallUpdateDamgeRecive _currenthealth)
        (Default|CallDead)
        (else
          (Default|CallUpdateDamgeRecive _currenthealth))))))

(fn GetInitHealthData
  (return (Variables|Default|GetMaxHealth) (Variables|Default|GetCurrentHealth)))